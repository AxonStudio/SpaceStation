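; BP_SmartFridge is an interactable fridge device that dispenses and takes back cans while tracking a count.
; Interact asks BPHoles to output a BP_UselessCan at the Cube14 mesh, then decrements the count with no lower limit.
; Any actor entering the Box, except the first-person character, goes to BPHoles input and increments the count, whether or not it is a can.
; Both paths print the new count.
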(event OnComponentBeginOverlap(Box)
  (params (OverlappedComponent :type Primitive%20Component%20Object%20Reference) (OtherActor :type Actor%20Object%20Reference) (OtherComp :type Primitive%20Component%20Object%20Reference) (OtherBodyIndex :type Integer) (bFromSweep :type Boolean) (SweepResult :type Hit%20Result%20Structure%20%28by%20ref%29))
  ;[0.15 0.15 0.15 0.5] The destruction of a can
  (Utilities|Casting|CastToBP_FirstPersonCharacter OtherActor
    (:CastFailed
      (Default|Input (Variables|Default|GetBP_Holes) OtherActor)
      (bind _output_get (Variables|Default|SetCans (+ (Variables|Default|GetCans) 1)))
      (Development|PrintString (Utilities|String|ToString(Integer) _output_get)))))

(event EventBeginPlay)

(event Collision|EventActorBeginOverlap
  (params (OtherActor :type Actor%20Object%20Reference)))

(event EventTick
  (params (DeltaSeconds :type Float%20%28single-precision%29)))

(event EventInteract
  ;[0.15 0.15 0.15 0.5] The creation of a can
  (Default|Output (Variables|Default|GetBP_Holes) "/Game/Project/Blueprints/Items/BP_UselessCan.BP_UselessCan_C" (Variables|Default|GetCube14))
  (bind _output_get (Variables|Default|SetCans (- (Variables|Default|GetCans) 1)))
  (Development|PrintString (Utilities|String|ToString(Integer) _output_get)))

(fn ConstructionScript)