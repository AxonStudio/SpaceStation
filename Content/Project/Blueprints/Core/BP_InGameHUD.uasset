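; BP_InGameHUD is the in-game HUD Blueprint that owns and toggles the pause menu.
; On BeginPlay it creates WBP_Pause with a reference to itself and adds it to the viewport collapsed.
; TogglePauseMenu branches on the widget's visibility to show or collapse it, switching mouse cursor, UI-only or game-only input mode, and game pause state together.
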(event EventBeginPlay
  (bind _returnvalue (UserInterface|CreateWidget "/Game/Project/UI/PauseMenu/WBP_Pause.WBP_Pause_C" 0 self))
  (bind _output_get (Variables|Default|SetWBP_Pause _returnvalue))
  (Widget|SetVisibility _output_get "Collapsed")
  (UserInterface|Viewport|AddtoViewport _output_get 0))

(fn ConstructionScript)

(fn TogglePauseMenu
  (bind _returnvalue (Game|GetPlayerController 0))
  (bind _returnvalue_2 (Game|GetPlayerController 0))
  (bind _wbp_pause (Variables|Default|GetWBP_Pause))
  (switch Utilities|FlowControl|Switch|SwitchonESlateVisibility (Widget|GetVisibility (Variables|Default|GetWBP_Pause))
    (:Visible
      (Variables|/Script/UMG.Widget|SetVisibility _wbp_pause "Collapsed")
      (Variables|/Script/Engine.PlayerController|SetbShowMouseCursor _returnvalue_2 false)
      (Input|SetInputModeGameOnly _returnvalue_2 false)
      (Game|SetGamePaused false))
    (:Collapsed
      (Variables|/Script/UMG.Widget|SetVisibility _wbp_pause "Visible" :!label _label)
      (Variables|/Script/Engine.PlayerController|SetbShowMouseCursor _returnvalue true)
      (Input|SetInputModeUIOnly _returnvalue 0 "DoNotLock" false)
      (Game|SetGamePaused true))
    (:Hidden
      (goto _label))))