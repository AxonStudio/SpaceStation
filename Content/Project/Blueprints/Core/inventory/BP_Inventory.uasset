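; BP_Inventory holds the player's item slots and drives the inventory screen.
; On BeginPlay it adds the input mapping, creates WB_Inventory, sizes Slots and passes itself to the widget's item panel.
; IA_Inventory toggles the widget, switching to UI-only input with cursor on opening, with no restore on closing.
; AddItemToInventory merges into a same-row stack within DT_Item's StackSize, otherwise fills the first empty slot, returning false if none.
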(event Input|EnhancedActionEvents|EnhancedInputActionIA_Inventory
  (params (ActionValue :type Boolean) (ElapsedSeconds :type Float%20%28double-precision%29) (TriggeredSeconds :type Float%20%28double-precision%29) (InputAction :type Input%20Action%20Object%20Reference :default "/Game/Project/Blueprints/Core/inventory/IA_Inventory.IA_Inventory"))
  (bind _returnvalue (Game|GetPlayerController 0))
  (:Started
    (if (Widget|IsVisible (Variables|Default|GetInventory))
      (Widget|RemovefromParent (Variables|Default|GetInventory))
      (else
        (Variables|/Script/Engine.PlayerController|SetbShowMouseCursor _returnvalue true)
        (Input|SetInputModeUIOnly _returnvalue (Variables|Default|GetInventory) "DoNotLock" false)
        (UserInterface|Viewport|AddtoViewport (Variables|Default|GetInventory) 0)))))

(event EventBeginPlay
  (bind _returnvalue (Game|GetPlayerController 0))
  (Utilities|IsValid _returnvalue
    (:Is%20Valid
      (Input|AddMappingContext (PlayerController|LocalPlayerSubsystems|GetEnhancedInputLocalPlayerSubsystem _returnvalue) "/Game/Project/Blueprints/Core/inventory/IMC_Inventory.IMC_Inventory" 0 "(bIgnoreAllPressedKeysUntilRelease=True,bForceImmediately=False,bNotifyUserSettings=False)")
      (bind _returnvalue_2 (UserInterface|CreateWidget "/Game/Project/Blueprints/Core/inventory/UI/WB_Inventory.WB_Inventory_C"))
      (bind _output_get (Variables|Default|SetInventory _returnvalue_2))
      (Utilities|Array|Resize (Variables|Default|GetSlots) (Variables|Default|GetSlotSize))
      (Default|LoadInventory (Variables|/Game/Project/Blueprints/Core/inventory/UI/WB_Inventory.WB_Inventory_C|GetWB_ItemInventory _output_get) self))))

(fn AddItemtoInventory
  (params (Item :type S%20Itemmaster%20Structure))
  (bind (_datatable _itemtype) (Utilities|Struct|BreakS_Itemmaster Item))
  (bind (_datatable_2 _itemtype_2 _count) (Utilities|Struct|BreakS_Itemmaster Item))
  ;[0.15 0.15 0.15 0.5] Проверка на схожий предмет в инвенторе и хватет ли место
  (for (_array_element _array_index) (Variables|Default|GetSlots)
    (if (== (.RowName (Utilities|Struct|BreakDataTableRowHandle (.datatable _array_element))) (.RowName (Utilities|Struct|BreakDataTableRowHandle (.DataTable (Utilities|Struct|BreakS_Itemmaster Item)))))
      (bind _returnvalue (Utilities|GetDataTableRow "/Game/Project/Blueprints/Core/inventory/DataTable/DT_Item.DT_Item" (.RowName (Utilities|Struct|BreakDataTableRowHandle _datatable_2)))
        (:then
          (if (>= (.StackSize (Utilities|Struct|BreakS_Item _returnvalue)) (+ (.count _array_element) _count))
            (Utilities|Array|SetArrayElem (Variables|Default|GetSlots) _array_index (Utilities|Struct|MakeS_Itemmaster _datatable _itemtype (+ (.count _array_element) _count)))
            (return true))))))
  ;[0.15 0.15 0.15 0.5] Проверка на пустой слот
  (for (_array_element_2 _array_index_2) (Variables|Default|GetSlots)
    (if (== (.count _array_element_2) 0)
      (Utilities|Array|SetArrayElem (Variables|Default|GetSlots) _array_index_2 Item)
      (return true)))
  (return false))