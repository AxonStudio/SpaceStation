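; BP_Item is a pickup item actor that the player can interact with to add it to their inventory.
; On construction, it sets its mesh from the data table row referenced by Itemdata and enables physics simulation.
; At BeginPlay it caches the first-person character's inventory.
; Interact runs the parent logic, tries to add Itemdata, and on success reloads the inventory widget and destroys the actor.
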(event EventBeginPlay
  ;[0.15 0.15 0.15 0.5] Получаем инвентарь
  (bind _asbp_first_person_character (Utilities|Casting|CastToBP_FirstPersonCharacter (Game|GetPlayerCharacter 0)))
  (Variables|Default|SetBP_Inventory (Variables|/Game/FirstPerson/Blueprints/BP_FirstPersonCharacter.BP_FirstPersonCharacter_C|GetBP_Inventory _asbp_first_person_character)))

(event EventInteract
  (bind _bp_inventory (Variables|Default|GetBP_Inventory))
  ;[0.15 0.15 0.15 0.5] Оброботка поподания
  (|CallParentFunction)
  (bind _additemtoinventory (Default|AddItemtoInventory _bp_inventory (Variables|Default|GetItemdata)))
  (if _additemtoinventory
    (Default|LoadInventory (Variables|/Game/Project/Blueprints/Core/inventory/UI/WB_Inventory.WB_Inventory_C|GetWB_ItemInventory (Variables|/Game/Project/Blueprints/Core/inventory/BP_Inventory.BP_Inventory_C|GetInventory _bp_inventory)) _bp_inventory)
    (Actor|DestroyActor)))

(fn ConstructionScript
  (bind _itemdata (Variables|Default|GetItemdata))
  (bind (_datatable _rowname) (Utilities|Struct|BreakDataTableRowHandle (.datatable _itemdata)))
  (|CallParentFunction)
  (bind _returnvalue (Utilities|GetDataTableRow _datatable _rowname)
    (:then
      (Components|StaticMesh|SetStaticMesh (Variables|Character|GetMesh) (.Mesh (Utilities|Struct|BreakS_Item _returnvalue)))
      (Physics|SetSimulatePhysics (Variables|Character|GetMesh) true))))