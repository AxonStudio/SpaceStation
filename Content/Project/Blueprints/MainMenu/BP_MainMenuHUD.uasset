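; BP_MainMenuHUD is the main menu HUD that creates and manages the menu, settings and creators screens.
; On BeginPlay it adds all three widgets to the viewport, with Settings and Creators collapsed, and shows the mouse cursor.
; ToggleSettings and ToggleCreators switch their panel between visible and collapsed, so the widgets are created once and only their visibility changes.
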(event EventBeginPlay
  (bind _returnvalue (UserInterface|CreateWidget "/Game/Project/UI/MainMenu/WBP_MainMenu.WBP_MainMenu_C"))
  (bind _output_get (Variables|Default|SetMainMenu _returnvalue))
  (UserInterface|Viewport|AddtoViewport _output_get 0)
  (bind _returnvalue_2 (UserInterface|CreateWidget "/Game/Project/UI/MainMenu/WBP_Settings.WBP_Settings_C"))
  (bind _output_get_2 (Variables|Default|SetSettings _returnvalue_2))
  (Widget|SetVisibility _output_get_2 "Collapsed")
  (UserInterface|Viewport|AddtoViewport _output_get_2 0)
  (bind _returnvalue_3 (UserInterface|CreateWidget "/Game/Project/UI/MainMenu/WBP_Creators.WBP_Creators_C"))
  (bind _output_get_3 (Variables|Default|SetCreators _returnvalue_3))
  (Widget|SetVisibility _output_get_3 "Collapsed")
  (UserInterface|Viewport|AddtoViewport _output_get_3 0)
  (Variables|/Script/Engine.PlayerController|SetbShowMouseCursor (Game|GetPlayerController 0) true))

(fn ConstructionScript)

(fn ToggleSettings
  (bind _settings (Variables|Default|GetSettings))
  (switch Utilities|FlowControl|Switch|SwitchonESlateVisibility (Widget|GetVisibility (Variables|Default|GetSettings))
    (:Visible
      (Widget|SetVisibility _settings "Collapsed"))
    (:Collapsed
      (Widget|SetVisibility _settings "Visible" :!label _label))
    (:Hidden
      (goto _label))))

(fn ToggleCreators
  (bind _creators (Variables|Default|GetCreators))
  (switch Utilities|FlowControl|Switch|SwitchonESlateVisibility (Widget|GetVisibility (Variables|Default|GetCreators))
    (:Visible
      (Widget|SetVisibility _creators "Collapsed"))
    (:Collapsed
      (Widget|SetVisibility _creators "Visible" :!label _label))
    (:Hidden
      (goto _label))))