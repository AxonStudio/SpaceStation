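; BP_InGameHUD is the in-game HUD Blueprint that manages opening and closing the pause menu.
; BeginPlay creates a WBP_Pause widget once and keeps a reference to it.
; OpenPauseMenu adds that widget to the viewport, shows the cursor, switches to UI-only input and pauses the game.
; ContinueGame reverses this by unpausing, hiding the cursor, restoring game-only input and removing the widget.
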(event EventBeginPlay
  (bind _returnvalue (UserInterface|CreateWidget "/Game/Project/UI/InGame/PauseMenu/WBP_Pause.WBP_Pause_C"))
  (Variables|Default|SetWBP_Pause _returnvalue))

(fn ConstructionScript)

(fn OpenPauseMenu
  (bind _returnvalue (Game|GetPlayerController 0))
  (UserInterface|Viewport|AddtoViewport (Variables|Default|GetWBP_Pause) 0)
  (Variables|/Script/Engine.PlayerController|SetbShowMouseCursor _returnvalue true)
  (Input|SetInputModeUIOnly _returnvalue 0 "DoNotLock" false)
  (Game|SetGamePaused true))

(fn ContinueGame
  (bind _returnvalue (Game|GetPlayerController 0))
  (Game|SetGamePaused false)
  (Variables|/Script/Engine.PlayerController|SetbShowMouseCursor _returnvalue false)
  (Input|SetInputModeGameOnly _returnvalue false)
  (Widget|RemovefromParent (Variables|Default|GetWBP_Pause)))