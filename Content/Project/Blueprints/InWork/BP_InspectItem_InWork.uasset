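; Interactable item Blueprint that lets the player inspect its mesh up close and rotate it with the mouse.
; Interact runs once until reset, freezing movement and look, showing the cursor, and playing a timeline that lerps the mesh to the character's TestItemCharacter transform.
; While inspecting, mouse axis input adds local rotation to the mesh.
; Right mouse release restores controls, re-arms interaction and reverses the timeline to the transform cached at BeginPlay.
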(event EventInteract
  ;[0.15 0.15 0.15 0.5] Interaction
  (|CallParentFunction)
  (Utilities|FlowControl|DoOnce false
    (:Completed
      (Variables|/Script/Engine.PlayerController|SetbShowMouseCursor (Game|GetPlayerController 0) true)
      (Variables|Default|SetCanInspect?_0 true)
      (bind _asbp_first_person_character (Utilities|Casting|CastToBP_FirstPersonCharacter (Game|GetPlayerCharacter 0)))
      (Pawn|Components|CharacterMovement|DisableMovement (Variables|/Script/Engine.Character|GetCharacterMovement (Game|GetPlayerCharacter 0)))
      (Input|SetIgnoreLookInput (Game|GetPlayerController 0) true)
      (bind _newtrack_0 (Timeline|TimelineForSmooth PlayFromStart)
        (:Update
          (Transformation|SetWorldTransform (Variables|Default|GetMesh_0) (Math|Transform|MakeTransform (Math|Vector|Lerp(Vector) (Variables|Default|GetOriginalLocation_0) (.location (Transformation|GetWorldTransform (Variables|/Game/FirstPerson/Blueprints/BP_FirstPersonCharacter.BP_FirstPersonCharacter_C|GetTestItemCharacter _asbp_first_person_character))) _newtrack_0) (Math|Rotator|Lerp(Rotator) (Variables|Default|GetOriginalRotation_0) (.rotation (Transformation|GetWorldTransform (Variables|/Game/FirstPerson/Blueprints/BP_FirstPersonCharacter.BP_FirstPersonCharacter_C|GetTestItemCharacter _asbp_first_person_character))) _newtrack_0) "1.000000,1.000000,1.000000") false false))))))

(event EventBeginPlay
  (bind _mesh_0 (Variables|Default|GetMesh_0))
  ;[0.15 0.15 0.15 0.5] Set Default Location
  (Variables|Default|SetOriginalLocation_0 (Transformation|GetWorldLocation _mesh_0))
  (Variables|Default|SetOriginalRotation_0 (Transformation|GetWorldRotation _mesh_0))
  (Input|EnableInput (Game|GetPlayerController 0)))

(event EventTick
  (params (DeltaSeconds :type Float%20%28single-precision%29))
  ;[0.15 0.15 0.15 0.5] Mouse Inputs For Inspect
  (if (Variables|Default|GetCanInspect?_0)
    (Transformation|AddLocalRotation (Variables|Default|GetMesh_0) (Math|Rotator|MakeRotator (* (stale Input|MouseEvents|MouseX AxisValue) 0.4) (* (stale Input|MouseEvents|MouseY AxisValue) -0.4) 0.0) false false)))

(event Input|MouseEvents|MouseX
  (params (AxisValue :type Float%20%28single-precision%29))
  ;[0.15 0.15 0.15 0.5] Mouse Inputs For Inspect
  (if (Variables|Default|GetCanInspect?_0)
    (Transformation|AddLocalRotation (Variables|Default|GetMesh_0) (Math|Rotator|MakeRotator (* AxisValue 0.4) (* (stale Input|MouseEvents|MouseY AxisValue) -0.4) 0.0) false false)))

(event Input|MouseEvents|MouseY
  (params (AxisValue :type Float%20%28single-precision%29))
  ;[0.15 0.15 0.15 0.5] Mouse Inputs For Inspect
  (if (Variables|Default|GetCanInspect?_0)
    (Transformation|AddLocalRotation (Variables|Default|GetMesh_0) (Math|Rotator|MakeRotator (* (stale Input|MouseEvents|MouseX AxisValue) 0.4) (* AxisValue -0.4) 0.0) false false)))

(event Input|MouseEvents|RightMouseButton
  (params (Key :type Key%20Structure))
  (bind _returnvalue (Game|GetPlayerController 0))
  ;[0.15 0.15 0.15 0.5] Interaction
  (:Released
    (Utilities|FlowControl|Sequence
      (:then_0
        (Utilities|FlowControl|DoOnce false) ; enters at Reset
      )
      (:then_1
        (Variables|Default|SetCanInspect?_0 false)
        (Pawn|Components|CharacterMovement|SetMovementMode (Variables|/Script/Engine.Character|GetCharacterMovement (Game|GetPlayerCharacter 0)) "MOVE_Walking" 0)
        (Variables|/Script/Engine.PlayerController|SetbShowMouseCursor _returnvalue false)
        (Input|ResetIgnoreLookInput _returnvalue)
        (Input|SetInputModeGameOnly _returnvalue false)
        (bind _newtrack_0 (Timeline|TimelineForSmooth Reverse)
          (:Update
            (Transformation|SetWorldTransform (Variables|Default|GetMesh_0) (Math|Transform|MakeTransform (Math|Vector|Lerp(Vector) (Variables|Default|GetOriginalLocation_0) (.location (Transformation|GetWorldTransform (Variables|/Game/FirstPerson/Blueprints/BP_FirstPersonCharacter.BP_FirstPersonCharacter_C|GetTestItemCharacter (stale EventInteract _asbp_first_person_character)))) _newtrack_0) (Math|Rotator|Lerp(Rotator) (Variables|Default|GetOriginalRotation_0) (.rotation (Transformation|GetWorldTransform (Variables|/Game/FirstPerson/Blueprints/BP_FirstPersonCharacter.BP_FirstPersonCharacter_C|GetTestItemCharacter (stale EventInteract _asbp_first_person_character)))) _newtrack_0) "1.000000,1.000000,1.000000") false false)))))))

(fn ConstructionScript)