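; BP_HealthComponent is a health component that tracks current Health against a MaxHealth limit.
; On BeginPlay it calls FullHealth, which sets Health to MaxHealth.
; AddHP and SubtractHealth change Health by a given amount and clamp it so it never exceeds MaxHealth or drops below zero.
; It contains no death handling or change notifications.
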(event EventBeginPlay
  (CallFunction|FullHealth))

(fn AddHP
  (params (PlusHP :type Integer))
  ;[0.15 0.15 0.15 0.5] PlusHP
  (Variables|Default|SetHealth (+ (Variables|Default|GetHealth) PlusHP))
  ;[0.15 0.15 0.15 0.5] Doesn't allow you to exceed the maximum HP
  (if (> (Variables|Default|GetHealth) (Variables|Default|GetMaxHealth))
    (Variables|Default|SetHealth (Variables|Default|GetMaxHealth))))

(fn SubtractHealth
  (params (mINUShp :type Integer))
  ;[0.15 0.15 0.15 0.5] MinusHP
  (Variables|Default|SetHealth (- (Variables|Default|GetHealth) mINUShp))
  ;[0.15 0.15 0.15 0.5] Does not allow to make less than 0
  (if (< (Variables|Default|GetHealth) 0)
    (Variables|Default|SetHealth 0)))

(fn FullHealth
  (Variables|Default|SetHealth (Variables|Default|GetMaxHealth)))